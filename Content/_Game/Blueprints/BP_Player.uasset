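; Player character Blueprint with a MetaHuman-style modular body, a face mesh and an inventory component.
; The construction script makes the torso, legs and feet meshes follow the main mesh's pose via leader pose.
; On BeginPlay, if hair strands are unsupported, it copies opacity parameters from the high-LOD eyelash material to the fused eyelash material for lower LODs.
; A debug key adds stone items to the inventory through a server call.
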(event EventBeginPlay
  (CallFunction|HairLODSetup))

(event Collision|EventActorBeginOverlap
  (params (OtherActor :type Actor%20Object%20Reference)))

(event EventTick
  (params (DeltaSeconds :type Float%20%28single-precision%29)))

(event Input|KeyboardEvents|DebugKeyT
  (params (Key :type Key%20Structure :default "None") (ActionValue :type Input%20Action%20Value%20Structure))
  (:Pressed
    (Default|AddItemSERVER (Variables|Default|GetBPC_Inventory) (CallFunction|MakeItemtoAdd "/Game/_Game/InventorySystem/Items/DA_Stone.DA_Stone" 10))))

(fn ConstructionScript
  (Components|SkinnedMesh|SetLeaderPoseComponent (Variables|Default|GetTorsoMesh) (Variables|Character|GetMesh) false false))

(fn HairLODSetup
  (bind _returnvalue (Class|GroomBlueprintLibrary|IsHairStrandsSupportedinWorld))
  (if (not _returnvalue) ; If strands are disabled then make fused eyelashes visible on lower LODs
    (bind _as머티리얼_인스턴스_다이내믹 (Utilities|Casting|CastToMaterialInstanceDynamic (Class|PrimitiveComponent|GetMaterialbyName (Variables|Default|GetFace) (Variables|Default|GetEyelashes%20HiLOD%20Material%20Slot))))
    (bind _as머티리얼_인스턴스_다이내믹_2 (Utilities|Casting|CastToMaterialInstanceDynamic (Class|PrimitiveComponent|GetMaterialbyName (Variables|Default|GetFace) (Variables|Default|GetEyelashes%20Material%20%20Slot))))
    (bind _returnvalue_2 (Rendering|Material|GetScalarParameterValue _as머티리얼_인스턴스_다이내믹 "Opacity" :!class /Script/Engine.MaterialInstanceDynamic))
    (Rendering|Material|SetScalarParameterValue _as머티리얼_인스턴스_다이내믹_2 "Opacity" _returnvalue_2 :!class /Script/Engine.MaterialInstanceDynamic)
    (bind _returnvalue_3 (Rendering|Material|GetScalarParameterValue _as머티리얼_인스턴스_다이내믹 "OpacityRT" :!class /Script/Engine.MaterialInstanceDynamic))
    (Rendering|Material|SetScalarParameterValue _as머티리얼_인스턴스_다이내믹_2 "OpacityRT" _returnvalue_3 :!class /Script/Engine.MaterialInstanceDynamic)))